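; Player controller that drives Bp_Player with camera-relative movement, jumping and an orbit camera through Enhanced Input.
; On BeginPlay it sets game-only input, caches the pawn and its camera, and adds the gameplay mapping context.
; Movement follows the camera's forward and right vectors and writes a target yaw, offset 90 degrees, to the pawn.
; Look input rotates the spring arm with per-axis speeds and clamped pitch.
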(event Input|EnhancedActionEvents|EnhancedInputActionIA_Jump
  (params (ActionValue :type Boolean) (ElapsedSeconds :type Float%20%28double-precision%29) (TriggeredSeconds :type Float%20%28double-precision%29) (InputAction :type Input%20Action%20Object%20Reference :default "/Game/Imputs/IA_Jump.IA_Jump"))
  (bind _playerref (Variables|Default|GetPlayerRef)
    (:then
      (Character|Jump _playerref))
    (:else)))

(event Input|EnhancedActionEvents|EnhancedInputActionIA_movement
  (params (ActionValue :type Vector%202D%20Structure) (ElapsedSeconds :type Float%20%28double-precision%29) (TriggeredSeconds :type Float%20%28double-precision%29) (InputAction :type Input%20Action%20Object%20Reference :default "/Game/Imputs/IA_movement.IA_movement"))
  (bind (_x _y) (Math|Vector2D|BreakVector2D ActionValue))
  (bind _playerref (Variables|Default|GetPlayerRef)
    (:then
      (bind _playercamera (Variables|Default|GetPlayerCamera)
        (:then
          (Pawn|Input|AddMovementInput _playerref (+ (* (Math|Vector|GetForwardVector _playercamera) _x) (* (Math|Vector|GetRightVector _playercamera) _y)) 1.0 false)
          (Variables|/Game/Player/Bp_Player.Bp_Player_C|SetTraget_Rotaion%20 _playerref (- (.yaw (Math|Rotator|MakeRotfromX (Math|Vector|Normalize (+ (* (Math|Vector|GetForwardVector _playercamera) _x) (* (Math|Vector|GetRightVector _playercamera) _y))))) 9e+01)))
        (:else)))
    (:else)))

(event Input|EnhancedActionEvents|EnhancedInputActionIA_Camera
  (params (ActionValue :type Vector%202D%20Structure) (ElapsedSeconds :type Float%20%28double-precision%29) (TriggeredSeconds :type Float%20%28double-precision%29) (InputAction :type Input%20Action%20Object%20Reference :default "/Game/Imputs/IA_Camera.IA_Camera"))
  (CallFunction|MoveCamera ActionValue))

(event EventBeginPlay
  (CallFunction|EventTrack))

(fn ConstructionScript)

(fn EventTrack
  (Input|SetInputModeGameOnly self false)
  (bind _asbp_player (Utilities|Casting|CastToBp_Player (Pawn|GetControlledPawn)))
  (bind _output_get (Variables|Default|SetPlayerRef _asbp_player))
  (Variables|Default|SetPlayerCamera (Variables|/Game/Player/Bp_Player.Bp_Player_C|GetCamera _output_get))
  (Input|AddMappingContext (PlayerController|LocalPlayerSubsystems|GetEnhancedInputLocalPlayerSubsystem) "/Game/Imputs/IM_Gameplay.IM_Gameplay" 0 "(bIgnoreAllPressedKeysUntilRelease=True,bForceImmediately=False,bNotifyUserSettings=False)"))

(fn MoveCamera
  (params (InVec :type Vector%202D%20Structure))
  (bind (_x _y) (Math|Vector2D|BreakVector2D InVec))
  (bind _playerref (Variables|Default|GetPlayerRef)
    (:then
      (Transformation|SetRelativeRotation (Variables|/Game/Player/Bp_Player.Bp_Player_C|GetSpringArm _playerref) (Math|Rotator|MakeRotator 0.0 (Math|Float|Clamp(Float) (+ (.Pitch (Math|Rotator|BreakRotator (Variables|/Script/Engine.SceneComponent|GetRelativeRotation (Variables|/Game/Player/Bp_Player.Bp_Player_C|GetSpringArm _playerref)))) (* _y (Variables|Default|GetcamSpeedY))) (Variables|Default|GetminAngleY) (Variables|Default|GetmaxAngleY)) (+ (.Yaw (Math|Rotator|BreakRotator (Variables|/Script/Engine.SceneComponent|GetRelativeRotation (Variables|/Game/Player/Bp_Player.Bp_Player_C|GetSpringArm _playerref)))) (* _x (Variables|Default|GetcamSpeedX)))) false false))
    (:else)))