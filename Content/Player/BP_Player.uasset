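; BP_Player is the player character Blueprint, handling toggled crouch, a timed jab flag and mesh rotation.
; BeginPlay derives a target yaw from the camera, caches walk speed and binds capsule overlap; Tick interpolates the mesh toward that yaw.
; Helpers switch run speed, destroy overlapped BP_pick actors and print downward trace hit counts.
; Switch interaction and object toggling are mostly stubs, and several helpers are never called here.
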(event Input|EnhancedActionEvents|EnhancedInputActionIA_Agacharse
  (params (ActionValue :type Boolean) (ElapsedSeconds :type Float%20%28double-precision%29) (TriggeredSeconds :type Float%20%28double-precision%29) (InputAction :type Input%20Action%20Object%20Reference :default "/Game/Imputs/IA_Agacharse.IA_Agacharse"))
  (:Started
    (Utilities|FlowControl|FlipFlop
      (:A
        (Character|Crouch)
        (Variables|Default|SetisCrouching true))
      (:B
        (Character|UnCrouch)
        (Variables|Default|SetisCrouching false)))))

(event Input|EnhancedActionEvents|EnhancedInputActionIA_Jab
  (params (ActionValue :type Boolean) (ElapsedSeconds :type Float%20%28double-precision%29) (TriggeredSeconds :type Float%20%28double-precision%29) (InputAction :type Input%20Action%20Object%20Reference :default "/Game/Imputs/IA_Jab.IA_Jab"))
  (:Started
    (Variables|Default|SetPegando%20 true)
    (Utilities|FlowControl|Delay 0.5)
    (Variables|Default|SetPegando%20 false)))

(event EventBeginPlay
  (CallFunction|IntRotation)
  (Variables|Default|SetBaseSpeed (Variables|/Script/Engine.CharacterMovementComponent|GetMaxWalkSpeed (Variables|Character|GetCharacterMovement)))
  (Collision|BindEventtoOnComponentBeginOverlap (Variables|Collision|GetCapsuleComponent) (EventDispatchers|CreateEvent :!event OnCollisionEnter)))

(event EventTick
  (params (DeltaSeconds :type Float%20%28single-precision%29))
  (CallFunction|RotateMesh DeltaSeconds))

(fn ConstructionScript)

(fn IntRotation
  (Variables|Default|SetTraget_Rotaion%20 (- (.yaw (Math|Rotator|MakeRotfromX (Math|Vector|Normalize (Math|Vector|GetForwardVector (Variables|Components|GetCamera))))) 0.0))
  (Transformation|SetWorldRotation (Variables|Character|GetMesh) "0, 0, 0" false false))

(fn RotateMesh
  (params (NewParam :type Float%20%28double-precision%29))
  (Transformation|SetWorldRotation (Variables|Character|GetMesh) (Math|Interpolation|RInterpTo (Transformation|GetWorldRotation (Variables|Character|GetMesh)) (Math|Rotator|MakeRotator 0.0 0.0 (Variables|Default|GetTraget_Rotaion%20)) NewParam (Variables|Default|GetRotation_Speed)) false false))

(fn SetRunning
  (params (IsRunning :type Boolean))
  (bind _basespeed (Variables|Default|GetBaseSpeed))
  (Utilities|FlowControl|Sequence
    (:then_0
      (if IsRunning
        (LocalVariables|SetCurrtentSpeed (* _basespeed (Variables|Default|GetRunMultiplayer)))
        (else
          (LocalVariables|SetCurrtentSpeed _basespeed))))
    (:then_1
      (Variables|/Script/Engine.CharacterMovementComponent|SetMaxWalkSpeed (Variables|Character|GetCharacterMovement) (LocalVariables|GetCurrtentSpeed)))))

(fn OnCollisionEnter
  (params (OverlappedComponent :type Primitive%20Component%20Object%20Reference) (OtherActor :type Actor%20Object%20Reference) (OtherComp :type Primitive%20Component%20Object%20Reference) (OtherBodyIndex :type Integer) (bFromSweep :type Boolean) (SweepResult :type Hit%20Result%20Structure%20%28by%20ref%29))
  (Utilities|FlowControl|Sequence
    (:then_0
      (if (Class|GameplayStatics|ObjectIsA OtherActor "/Game/BP_pick.BP_pick_C")
        (Actor|DestroyActor OtherActor)))
    (:then_1
      (if (Class|GameplayStatics|ObjectIsA OtherActor "/Game/BP_Switch.BP_Switch_C")
        _))))

(fn Interact
  (Variables|Default|GetSwitchReach
    (:then)
    (:else)))

(fn ToggleObject)

(fn CheckPlatform
  (bind _returnvalue (Transformation|GetActorLocation))
  (bind _outhits (Collision|MultiLineTraceByChannel _returnvalue (+ _returnvalue "" (* (Variables|/Script/Engine.CapsuleComponent|GetCapsuleHalfHeight (Variables|Collision|GetCapsuleComponent)) -1.1)) "TraceTypeQuery1" false 0 "None"))
  (Development|PrintString (Utilities|String|ToString(Integer) (Utilities|Array|Length _outhits))))

(fn ActivatedObject
  (Variables|Default|SetActivated true))

(fn DesactivatedObject)